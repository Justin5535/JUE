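; BP_JueControllerStatics is a utility of static helpers for putting UI widgets on screen through the player's BP_JuePlayerController.
; Each push function casts player controller 0 and forwards the widget class to its RootLayout's Game, Menu or Modal push, returning the result.
; Only PushModal validates the class and prints an error on failure.
; AddWidgetToHUD is an unfinished TODO stub that only performs the cast.
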(fn `AddWidgetToHUD`
  (params (WidgetObject :type "Widget Object Reference"))
  (returns (ReturnValue :type "OverlaySlot Object Reference"))
  ; @TODO: Fill this in your gameplay controller
  (bind _asbp_jueplayer_controller (cast `/JUE/Core/Controllers/BP_JuePlayerController` (`GameplayStatics.GetPlayerController` WidgetObject))))

(fn `PushModal`
  (params (WidgetClass :type "CommonActivatableWidget Class Reference"))
  (returns (ReturnValue :type "CommonActivatableWidget Object Reference"))
  (if (`KismetSystemLibrary.IsValidClass` WidgetClass)
    (bind _asbp_jueplayer_controller (cast `/JUE/Core/Controllers/BP_JuePlayerController` (`GameplayStatics.GetPlayerController` null))
      (:`then`
        (bind _returnvalue (`/JUE/UI/WBP_Layout.PushWidgetToModal` (`/JUE/Core/Controllers/BP_JuePlayerController.RootLayout` _asbp_jueplayer_controller) WidgetClass))
        (return _returnvalue))
      (:`CastFailed`
        _)))
  (`KismetSystemLibrary.PrintString` null "ERROR: Tried to push Modal!")
  (return null))

(fn `PushWidgetToGame`
  (params (WidgetClass :type "CommonActivatableWidget Class Reference"))
  (returns (PushedWidget :type "CommonActivatableWidget Object Reference"))
  (bind _asbp_jueplayer_controller (cast `/JUE/Core/Controllers/BP_JuePlayerController` (`GameplayStatics.GetPlayerController` null))
    (:`then`
      (bind _returnvalue (`/JUE/UI/WBP_Layout.PushWidgetToGame` (`/JUE/Core/Controllers/BP_JuePlayerController.RootLayout` _asbp_jueplayer_controller) WidgetClass))
      (return _returnvalue))
    (:`CastFailed`
      (return null))))

(fn `PushWidgetToMenu`
  (params (WidgetClass :type "CommonActivatableWidget Class Reference"))
  (returns (ReturnValue :type "CommonActivatableWidget Object Reference"))
  (bind _asbp_jueplayer_controller (cast `/JUE/Core/Controllers/BP_JuePlayerController` (`GameplayStatics.GetPlayerController` null))
    (:`then`
      (bind _pushedwidget (`/JUE/UI/WBP_Layout.PushWidgetToMenu` (`/JUE/Core/Controllers/BP_JuePlayerController.RootLayout` _asbp_jueplayer_controller) WidgetClass))
      (return _pushedwidget))
    (:`CastFailed`
      (return null))))