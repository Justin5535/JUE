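; BP_JuePlayerController is a player controller that builds the root UI for the local player.
; On BeginPlay, for local controllers only, it creates a WBP_Layout widget and adds it to the player screen.
; It then pushes the optional DefaultUI class onto the layout's menu and, when CreateHUD is set, pushes WBP_HUD onto the game layer and stores the reference.
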(event `self.ReceiveBeginPlay`
  (bind _defaultui (`self.DefaultUI`))
  (`parent.ReceiveBeginPlay`)
  (if (`self.IsLocalPlayerController`)
    (bind _returnvalue (`|CreateWidget` "/JUE/UI/WBP_Layout.WBP_Layout_C" self))
    (bind _output_get (set `self.RootLayout` _returnvalue))
    (`UserWidget.AddToPlayerScreen` _output_get 0)
    (if (`KismetSystemLibrary.IsValidClass` _defaultui)
      (`/JUE/UI/WBP_Layout.PushWidgetToMenu` (`self.RootLayout`) _defaultui))
    (if (`self.CreateHUD`)
      (bind _returnvalue_2 (`/JUE/UI/WBP_Layout.PushWidgetToGame` (`self.RootLayout`) "/JUE/UI/WBP_HUD.WBP_HUD_C"))
      (bind _aswbp_hud (cast `/JUE/UI/WBP_HUD` _returnvalue_2))
      (set `self.HUD` _aswbp_hud))))

(fn `UserConstructionScript`)